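; AITest is a test AI pawn that moves to a supplied location while selected.
; Enabled toggles selection off when already selected, otherwise takes the passed value.
; CustomSet issues AI Move To and retries after a short delay on failure, or prints a debug string when unselected.
; AIMoving, called on BeginPlay, is empty, and the random-point and fixed-destination movement loop is left disconnected, as are empty Moving functions.
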(event Custom|AIMoving)

(event Custom|CustomSet
  (params (CustomLocation :type Vector))
  (if (Variables|Default|GetisSelected)
    (bind _output_get (Variables|Default|SetCustom%20Location CustomLocation))
    (AI|AIMoveTo self _output_get 0 5.0 false
      (:OnFail
        (Utilities|FlowControl|Delay 0.2)
        (CallFunction|CustomSet _output_get)))
    (else
      (Development|PrintString "Hello"))))

(event EventBeginPlay
  (CallFunction|AIMoving))

(event EventEnabled
  (params (isEnabled :type Boolean))
  (if (Variables|Default|GetisSelected)
    (Variables|Default|SetisSelected false)
    (else
      (Variables|Default|SetisSelected isEnabled))))

(fn ConstructionScript)

(fn Moving)

(fn CustomMoving
  (params (CustomLocation1 :type Vector)))