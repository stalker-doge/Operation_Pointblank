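; AIUnit is an AI unit Blueprint that wanders the navmesh on its own from BeginPlay.
; The Moving event picks a random navigable point near the unit's current location and sends it there with AI MoveTo.
; It then calls itself again after a pause, shorter on failure than on success, forming an endless roam loop.
; The Enabled function takes a flag but is an empty stub.
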(event EventBeginPlay
  (CallFunction|Moving))

(event Collision|EventActorBeginOverlap
  (params (OtherActor :type Actor%20Object%20Reference)))

(event EventTick
  (params (DeltaSeconds :type Float%20%28single-precision%29)))

(fn ConstructionScript)

(fn Enabled
  (params (isEnabled :type Boolean))
  (return))

(event Custom|Moving
  (bind _output_get (Variables|Default|SetRandom%20Location (.RandomLocation (Class|NavigationSystemV1|GetRandomPointinNavigableRadius (Transformation|GetActorLocation) 4e+02 0 0))))
  (AI|AIMoveTo self _output_get 0 5.0 false
    (:OnSuccess
      (Utilities|FlowControl|Delay 1.0))
    (:OnFail
      (Utilities|FlowControl|Delay 0.2)))
  (CallFunction|Moving))