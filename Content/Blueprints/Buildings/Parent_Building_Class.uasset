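; Base building class for an RTS-style game that can be selected and produces units from a queue.
; Selection toggles a decal and a BuildingsUI widget, created on BeginPlay and filled with the building's action buttons.
; A looping timer advances production progress using each unit class's default production time, spawns the finished unit at the spawn point, then takes the next queued class.
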(event Custom|Add%20Unit%20to%20Queue
  (params (Unit :type My%20Unit%20AI%20Class%20Reference))
  (Utilities|Array|Add (Variables|Default|GetUnitProductionQueue) Unit))

(event Custom|ProcessProductionQueue
  (if (Variables|Default|GetisProducingUnit)
    (bind _output_get (Variables|Default|SetProductionTimeSpent (+ (Variables|Default|GetProductionTimeSpent) (Variables|Default|GetProductionGranularity))))
    (bind _output_get_2 (Variables|Default|SetProductionProgress (/ _output_get (Variables|Default|GetProductionTimeNeeded))))
    (if (>= _output_get_2 1.0)
      (Game|SpawnActorfromClass (Variables|Default|GetUnit%20Being%20Produced) (Math|Transform|MakeTransform (Transformation|GetWorldLocation (Variables|Default|GetUnitSpawnPoint)) "0, 0, 0" "1,1,1") "AdjustIfPossibleButAlwaysSpawn" 0 0)
      (Variables|Default|SetProductionProgress 0.0)
      (Variables|Default|SetProductionTimeSpent 0.0)
      (Variables|Default|SetUnit%20Being%20Produced 0)
      (Variables|Default|SetisProducingUnit false))
    (elif (> (Utilities|Array|Length (Variables|Default|GetUnitProductionQueue)) 0)
      (bind _output_get_3 (Variables|Default|SetUnit%20Being%20Produced (Utilities|Array|Get(acopy) (Variables|Default|GetUnitProductionQueue))))
      (Variables|Default|SetProductionTimeNeeded (.ProductionTime (Utilities|GetClassDefaults _output_get_3)))
      (Utilities|Array|RemoveIndex (Variables|Default|GetUnitProductionQueue))
      (Variables|Default|SetisProducingUnit true))))

(event EventSelectThis
  (Rendering|SetVisibility (Variables|Default|GetSelectedDecal) true false)
  (UserInterface|Viewport|AddtoViewport (Variables|Default|GetBuildingSelectedWidget) 0))

(event EventDeselectThis
  (Rendering|SetVisibility (Variables|Default|GetSelectedDecal) false false)
  (Widget|RemovefromParent (Variables|Default|GetBuildingSelectedWidget)))

(event EventBeginPlay
  (Utilities|FlowControl|Sequence
    (:then_0
      (bind _returnvalue (UserInterface|CreateWidget "/Game/Blueprints/Buildings/BuildingsUI.BuildingsUI_C"))
      (Variables|Default|SetBuildingSelectedWidget _returnvalue)
      (Variables|/Game/Blueprints/Buildings/BuildingsUI.BuildingsUI_C|SetBuildingReference _returnvalue self)
      (for _array_element (Variables|Default|GetActionBoxButtons)
        (Class|WrapBox|AddChildtoWrapBox (Variables|/Game/Blueprints/Buildings/BuildingsUI.BuildingsUI_C|GetActionBox (Variables|Default|GetBuildingSelectedWidget)) _array_element)))
    (:then_2
      (Utilities|Time|SetTimerbyEvent (delegate Custom|ProcessProductionQueue) (Variables|Default|GetProductionGranularity) true))))

(fn ConstructionScript)

(fn GrabSelectedUnits
  (return 0))