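; EnemyAI is an enemy pawn Blueprint that chases the nearest AITest actor.
; BeginPlay caches all AITest actors in UnitArray.
; Each Tick scans that array by 2D distance, issuing AIMoveTo whenever one beats the stored ClosestDistance, which resets to a large value only when a move succeeds.
; The Moving and CustomMoving functions are empty stubs.
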(event EventBeginPlay
  (bind _outactors (Actor|GetAllActorsOfClass "/Game/Blueprints/AITest.AITest_C"))
  (Variables|Default|SetUnitArray _outactors))

(event EventTick
  (params (DeltaSeconds :type Float%20%28single-precision%29))
  (for _array_element (Variables|Default|GetUnitArray)
    (if (< (Math|Vector|Distance2D(Vector) (Transformation|GetActorLocation _array_element) (Transformation|GetActorLocation)) (Variables|Default|GetClosestDistance))
      (Variables|Default|SetClosestDistance (Math|Vector|Distance2D(Vector) (Transformation|GetActorLocation _array_element) (Transformation|GetActorLocation)))
      (Variables|Default|SetCustom%20Location (Transformation|GetActorLocation _array_element))
      (AI|AIMoveTo self (Variables|Default|GetCustom%20Location) 0 1e+01 false
        (:OnSuccess
          (Variables|Default|SetClosestDistance 9e+05))))))

(fn ConstructionScript)

(fn Moving)

(fn CustomMoving
  (params (CustomLocation1 :type Vector)))