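; RTS HUD that draws a marquee selection box and selects MyUnitAI units inside it.
; Marquee press, hold and release events track the mouse corners and drawing state.
; While drawing, each DrawHUD messages units in the rectangle to select and records them in SelectedUnits.
; Recorded units outside it get deselect messages but stay in the array, as the Remove node never runs.
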(event EventMarqueePressed
  (bind _returnvalue (Game|GetPlayerController 0))
  (bind (_locationx _locationy) (Game|Player|GetMousePosition _returnvalue))
  (Variables|Default|SetisDrawing true)
  (bind _output_get (Variables|Default|SetStartMousePosition (Math|Vector2D|MakeVector2D _locationx _locationy)))
  (Variables|Default|SetCurrentMousePosition _output_get))

(event EventMarqueeHeld
  (bind _returnvalue (Game|GetPlayerController 0))
  (bind (_locationx _locationy) (Game|Player|GetMousePosition _returnvalue))
  (Variables|Default|SetCurrentMousePosition (Math|Vector2D|MakeVector2D _locationx _locationy)))

(event EventMarqueeReleased
  (Variables|Default|SetisDrawing false))

(event EventDrawHUD
  (params (SizeX :type Integer) (SizeY :type Integer))
  (bind _startmouseposition (Variables|Default|GetStartMousePosition))
  (bind _currentmouseposition (Variables|Default|GetCurrentMousePosition))
  (bind _startmouseposition_2 (Variables|Default|GetStartMousePosition))
  (bind _currentmouseposition_2 (Variables|Default|GetCurrentMousePosition))
  (bind _outactors (Class|HUD|GetActorsinSelectionRectangle "/Game/Blueprints/MyUnitAI.MyUnitAI_C" _currentmouseposition_2 _startmouseposition_2 false false))
  (if (Variables|Default|GetisDrawing)
    (HUD|DrawRect "(R=0.000000,G=0.065139,B=0.895833,A=0.200000)" (.x _startmouseposition) (.y _startmouseposition) (- (.x _currentmouseposition) (.x _startmouseposition)) (- (.y _currentmouseposition) (.y _startmouseposition)))
    (Variables|Default|SetActors%20in%20rectangle _outactors)
    (for _array_element _outactors
      (Class|RTSInterface|SelectUnit(Message) _array_element)
      (Utilities|Array|AddUnique (Variables|Default|GetselectedUnits) _array_element))
    (for _array_element_2 (Variables|Default|GetselectedUnits)
      (if (== (Utilities|Array|FindItem (Variables|Default|GetActors%20in%20rectangle) _array_element_2) -1)
        (Class|RTSInterface|DeselectUnit(Message) _array_element_2)))))

(fn ConstructionScript)