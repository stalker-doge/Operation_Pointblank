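; LevelHandler is a Blueprint that moves the game through numbered levels and on to a win map.
; On BeginPlay it parses the current level number from a map name containing "Level".
; NextLevel increments that number and opens the matching map by built name, then sets FinalLevel once the number reaches a hard-coded threshold.
; When FinalLevel is already true, NextLevel opens GameWin instead.
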(event Custom|NextLevel
  (if (Variables|Default|GetFinalLevel)
    (Game|OpenLevel(byObjectReference) "/Game/Maps/GameWin.GameWin")
    (else
      (bind _result (Math|Integer|IncrementInt (Variables|Default|GetCurrentLevel))
        (:%20%20
          (Game|OpenLevel(byName) (Utilities|String|StringToName (Utilities|String|BuildString(Integer) "Level" "" _result)))
          (if (>= (Variables|Default|GetCurrentLevel) 3)
            (Variables|Default|SetFinalLevel true)))))))

(event EventBeginPlay
  (bind _returnvalue (Game|GetCurrentLevelName true))
  (if (Utilities|String|Contains _returnvalue "Level")
    (Variables|Default|SetCurrentLevel (Math|Conversions|ToInteger(Byte) (Utilities|String|RightChop _returnvalue 5)))))