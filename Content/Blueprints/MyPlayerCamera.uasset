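; MyPlayerCamera is a player camera actor that pans across the world when the mouse cursor nears a screen edge.
; The MouseX and MouseY input events normalize cursor position against viewport size and test for the outer two percent on each side.
; Left and right edges offset the actor along world Y, top and bottom along world X, at ScrollSpeed scaled by delta time.
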(event Input|MouseEvents|MouseX
  (params (AxisValue :type Float%20%28single-precision%29))
  (bind _returnvalue (Game|GetPlayerController 0))
  (bind _returnvalue_2 (Viewport|GetViewportSize))
  (bind _returnvalue_3 (Utilities|Time|GetWorldDeltaSeconds))
  (bind _scroll_speed (Variables|Default|GetScroll%20Speed))
  (bind _locationx (Game|Player|GetMousePosition _returnvalue))
  (bind _returnvalue_4 (* _scroll_speed _returnvalue_3))
  (bind _returnvalue_5 (/ _locationx (.x _returnvalue_2)))
  (if (> _returnvalue_5 0.98)
    (Transformation|AddActorWorldOffset (Math|Vector|MakeVector 0.0 _returnvalue_4 0.0))
    (elif (< _returnvalue_5 0.02)
      (Transformation|AddActorWorldOffset (Math|Vector|MakeVector 0.0 (* _returnvalue_4 -1.0) 0.0)))))

(event Input|MouseEvents|MouseY
  (params (AxisValue :type Float%20%28single-precision%29))
  (bind _returnvalue (Game|GetPlayerController 0))
  (bind _returnvalue_2 (Utilities|Time|GetWorldDeltaSeconds))
  (bind _returnvalue_3 (Viewport|GetViewportSize))
  (bind _scroll_speed (Variables|Default|GetScroll%20Speed))
  (bind _locationy (Game|Player|GetMousePosition _returnvalue))
  (bind _returnvalue_4 (* _scroll_speed _returnvalue_2))
  (bind _returnvalue_5 (/ _locationy (.y _returnvalue_3)))
  (if (> _returnvalue_5 0.98)
    (Transformation|AddActorWorldOffset (Math|Vector|MakeVector (* _returnvalue_4 -1.0) 0.0 0.0))
    (elif (< _returnvalue_5 0.02)
      (Transformation|AddActorWorldOffset (Math|Vector|MakeVector _returnvalue_4 0.0 0.0)))))

(fn ConstructionScript)