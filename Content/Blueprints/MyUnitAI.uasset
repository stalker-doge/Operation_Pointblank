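; Selectable unit Blueprint that moves itself to an ordered location through AI navigation.
; Enabled toggles selection off when the unit is already selected, otherwise applies the passed flag.
; CustomSetLocation stores the target and runs AIMoveTo only while selected, retrying after a short delay when the move fails.
; The AIMoving function and construction script are empty.
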(event Custom|CustomSetLocation
  (params (CustomLocation :type Vector))
  (bind _self self)
  (if (Variables|Default|GetisSelected)
    (bind _output_get (Variables|Default|SetCustom%20Location CustomLocation))
    (AI|AIMoveTo _self _output_get 0 5.0 false
      (:OnFail
        (Utilities|FlowControl|Delay 0.2)
        (CallFunction|CustomSetLocation _self _output_get)))))

(event EventEnabled
  (params (isEnabled :type Boolean))
  (if (Variables|Default|GetisSelected)
    (Variables|Default|SetisSelected false)
    (else
      (Variables|Default|SetisSelected isEnabled))))

(fn ConstructionScript)

(fn AIMoving)