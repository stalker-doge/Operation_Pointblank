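; Base resource point actor that captures over time while a capture-capable actor overlaps it.
; A looping timer advances progress, then flags it captured, sends a resource message to player controller 0 and resets progress.
; The timer keeps looping after completion until any actor ends overlap or a capable one re-enters.
; Tick passes self to the CaptureProgress widget; selection, capture-check and resource functions return empty defaults.
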(event Custom|SetCaptured
  (bind _output_get (Variables|Default|SetCapturePercent (+ (Variables|Default|GetCapturePercent) (Variables|Default|GetCaptureGranularity))))
  (bind _output_get_2 (Variables|Default|SetCaptureProgress (/ _output_get (Variables|Default|GetCaptureTimeNeeded))))
  (if (>= _output_get_2 1.0)
    (Variables|Default|SetHasBeenCaptured true)
    (Class|RTSInterface|AddResource(Message) (Game|GetPlayerController 0) "NewEnumerator0")
    (Variables|Default|SetCapturePercent 0.0)
    (Variables|Default|SetCaptureProgress 0.0)))

(event Collision|EventActorBeginOverlap
  (params (OtherActor :type Actor%20Object%20Reference))
  (bind _cancapture (Class|RTSInterface|CanCapture(Message) OtherActor))
  (if _cancapture
    (if (Variables|Default|GetHasBeenCaptured)
      (Utilities|Time|ClearandInvalidateTimerbyHandle (stale _returnvalue))
      (else
        (bind _returnvalue (Utilities|Time|SetTimerbyEvent (delegate Custom|SetCaptured) (Variables|Default|GetCaptureGranularity) true))))))

(event Collision|EventActorEndOverlap
  (params (OtherActor :type Actor%20Object%20Reference))
  (bind _cancapture (Class|RTSInterface|CanCapture(Message) OtherActor))
  (if _cancapture
    _
    (else
      _))
  (Utilities|Time|ClearandInvalidateTimerbyHandle (stale Collision|EventActorBeginOverlap _returnvalue)))

(event EventTick
  (params (DeltaSeconds :type Float%20%28single-precision%29))
  (bind _ascapture_progress (Utilities|Casting|CastToCaptureProgress (UserInterface|GetUserWidgetObject (Variables|Default|GetProgress))))
  (Variables|/Game/Blueprints/HUD/CaptureProgress.CaptureProgress_C|SetCapturePoint _ascapture_progress self))

(event EventBeginPlay
  (Variables|Default|SetProgressBar 0))

(fn ConstructionScript)

(fn CanCapture
  (return false))

(fn GrabSelectedEnemies
  (return 0))

(fn GrabSelectedUnits
  (return 0))

(fn ResourceKeeper
  (return 0.0 0.0 0.0))