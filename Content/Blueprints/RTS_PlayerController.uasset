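; RTS player controller Blueprint that feeds left-mouse input to the HUD for marquee (box) selection.
; On BeginPlay it sets Game and UI input mode with the cursor shown and locked to the viewport.
; Left mouse press and release toggle a held flag and send marquee pressed and released messages to the HUD.
; While the flag is set, Tick sends a held message every frame.
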(event EventBeginPlay
  (bind _returnvalue (Game|GetPlayerController 0))
  (Input|EnableInput _returnvalue)
  (Input|SetInputModeGameandUI _returnvalue 0 "LockAlways" false)
  (Variables|Default|SetbShowMouseCursor true))

(event EventTick
  (params (DeltaSeconds :type Float%20%28single-precision%29))
  (if (Variables|Default|GetisLeftMousePressed)
    (Class|RTSInterface|MarqueeHeld(Message) (HUD|GetHUD))))

(event Input|MouseEvents|LeftMouseButton
  (params (Key :type Key%20Structure :default "None"))
  (bind _returnvalue (HUD|GetHUD))
  (:Pressed
    (Variables|Default|SetisLeftMousePressed true)
    (Class|RTSInterface|MarqueePressed(Message) _returnvalue))
  (:Released
    (Variables|Default|SetisLeftMousePressed false)
    (Class|RTSInterface|MarqueeReleased(Message) _returnvalue)))

(fn ConstructionScript)