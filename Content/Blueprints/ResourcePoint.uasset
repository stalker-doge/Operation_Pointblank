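; ResourcePoint is a capturable point that accumulates Ammo once an AITest unit has held it.
; Overlap by the first AITest actor, looked up every Tick, starts a five-second Unit_Capture timer, and leaving clears it.
; Capture sets UnitPresent, which nothing here resets, so Ammo then rises every frame.
; BeginPlay also adds a Resources tracker widget to the viewport, though this graph never passes it Ammo.
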(event EventBeginPlay
  (bind _returnvalue (UserInterface|CreateWidget "/Game/Blueprints/HUD/Resources.Resources_C" (Game|GetPlayerController 0)))
  (bind _output_get (Variables|Default|SetResource%20tracker _returnvalue))
  (UserInterface|Viewport|AddtoViewport _output_get 0))

(event Collision|EventActorBeginOverlap
  (params (OtherActor :type Actor%20Object%20Reference))
  (if (== OtherActor (stale EventTick _returnvalue))
    (bind _returnvalue (Utilities|Time|SetTimerbyFunctionName self "Unit_Capture" 5.0))))

(event EventTick
  (params (DeltaSeconds :type Float%20%28single-precision%29))
  (bind _returnvalue (Actor|GetActorOfClass "/Game/Blueprints/AITest.AITest_C"))
  (if (Variables|Default|GetUnitPresent)
    (Math|Integer|IncrementInt (Variables|Default|GetAmmo))))

(event Collision|EventActorEndOverlap
  (params (OtherActor :type Actor%20Object%20Reference))
  (if (== (stale EventTick _returnvalue) OtherActor)
    (Utilities|Time|ClearandInvalidateTimerbyHandle (stale Collision|EventActorBeginOverlap _returnvalue))))

(fn ConstructionScript)

(fn UnitCapture
  (Variables|Default|SetUnitPresent true))