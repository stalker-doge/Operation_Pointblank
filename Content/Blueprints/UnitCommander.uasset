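; UnitCommander is a mouse-driven controller for selecting and commanding AITest units, taking player input and game-only input mode on BeginPlay.
; Left click, sharing logic with BroadcastLocation, traces under the cursor by object type and calls Enabled on the hit unit, never disabling others.
; Right click passes the cursor's visibility-trace location to every AITest unit through CustomSet.
; Its own Enabled function is an empty stub.
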(event Custom|BroadcastLocation
  (params (Cursor%20Location :type Vector%20%28by%20ref%29))
  (bind _array (Utilities|Array|MakeArray "ObjectTypeQuery7"))
  (bind _hitresult (Class|PlayerController|GetHitResultUnderCursorforObjects _array true))
  (bind (_bblockinghit _binitialoverlap _time _distance _location _impactpoint _normal _impactnormal _physmat _hitactor) (Collision|BreakHitResult _hitresult))
  (Variables|Default|SetCursor%20Location (.Location (Collision|BreakHitResult (.HitResult (Game|Player|GetHitResultUnderCursorbyChannel "TraceTypeQuery1" true)))))
  (Development|PrintString (Utilities|String|ToString(Vector) _location))
  (bind _outactors (Actor|GetAllActorsOfClass "/Game/Blueprints/AITest.AITest_C"))
  (for _array_element _outactors
    (if (== _array_element _hitactor)
      (CallFunction|Enabled _array_element (== _array_element _hitactor)))))

(event EventBeginPlay
  (bind _returnvalue (Game|GetPlayerController 0))
  (Input|EnableInput _returnvalue)
  (Input|SetInputModeGameOnly _returnvalue)
  (Class|GameplayStatics|SetViewportMouseCaptureMode "CapturePermanently"))

(event EventTick
  (params (DeltaSeconds :type Float%20%28single-precision%29)))

(event Input|MouseEvents|RightMouseButton
  (params (Key :type Key%20Structure :default "None"))
  (:Pressed
    (bind _output_get (Variables|Default|SetCursor%20Location (.Location (Collision|BreakHitResult (.HitResult (Game|Player|GetHitResultUnderCursorbyChannel "TraceTypeQuery1" true))))))
    (bind _outactors (Actor|GetAllActorsOfClass "/Game/Blueprints/AITest.AITest_C"))
    (for _array_element _outactors
      (Default|CustomSet _array_element _output_get))))

(event Input|MouseEvents|LeftMouseButton
  (params (Key :type Key%20Structure :default "None"))
  (bind _array (Utilities|Array|MakeArray "ObjectTypeQuery7"))
  (bind _hitresult (Class|PlayerController|GetHitResultUnderCursorforObjects _array true))
  (bind (_bblockinghit _binitialoverlap _time _distance _location _impactpoint _normal _impactnormal _physmat _hitactor) (Collision|BreakHitResult _hitresult))
  (:Pressed
    (Variables|Default|SetCursor%20Location (.Location (Collision|BreakHitResult (.HitResult (Game|Player|GetHitResultUnderCursorbyChannel "TraceTypeQuery1" true)))))
    (Development|PrintString (Utilities|String|ToString(Vector) _location))
    (bind _outactors (Actor|GetAllActorsOfClass "/Game/Blueprints/AITest.AITest_C"))
    (for _array_element _outactors
      (if (== _array_element _hitactor)
        (CallFunction|Enabled _array_element (== _array_element _hitactor))))))

(fn ConstructionScript)

(fn Enabled
  (params (isEnabled :type Boolean))
  (return))