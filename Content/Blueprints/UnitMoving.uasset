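; Player-controller style Blueprint intended to move the controlled pawn to the point under the cursor while left mouse is held.
; Moving, called on BeginPlay, passes a mouse-toggled Gate, traces under the cursor, runs AIMoveTo, then re-calls itself after a delay on success or failure.
; Pressing only opens the Gate without re-entering Moving.
; AIMoveTo receives the controlled pawn as TargetActor, with no Pawn input set.
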(event EventBeginPlay
  (CallFunction|Moving))

(event Collision|EventActorBeginOverlap
  (params (OtherActor :type Actor%20Object%20Reference)))

(event EventTick
  (params (DeltaSeconds :type Float%20%28single-precision%29)))

(fn ConstructionScript)

(event Custom|Moving
  (Utilities|FlowControl|Gate true
    (:Exit
      (Utilities|FlowControl|Delay 0.2)
      (bind _output_get (Variables|Default|SetRandom%20Location (.Location (Collision|BreakHitResult (.HitResult (Game|Player|GetHitResultUnderCursorbyChannel "TraceTypeQuery1" true))))))
      (AI|AIMoveTo 0 _output_get (Pawn|GetControlledPawn) 5.0 false
        (:OnSuccess
          (Utilities|FlowControl|Delay 1.0))
        (:OnFail
          (Utilities|FlowControl|Delay 0.2)))
      (CallFunction|Moving))))

(event Input|MouseEvents|LeftMouseButton
  (params (Key :type Key%20Structure :default "None"))
  (:Pressed
    (Utilities|FlowControl|Gate true) ; enters at Open
  )
  (:Released
    (Utilities|FlowControl|Gate true) ; enters at Close
  ))