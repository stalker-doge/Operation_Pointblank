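; Enemy unit that automatically hunts and shoots player units, falling back to buildings when none remain.
; BeginPlay links the health bar, gathers all MyUnitAI actors and starts a looping fire timer; production and destruction events update that list.
; Tick moves it toward the closest tracked target via AIMoveTo and destroys it once health drops below zero.
; The timer line-traces at the nearest in-range target, sending damage to whatever it hits.
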(event Custom|ShootUnit
  (bind _capsulecomponent (Variables|Default|GetCapsuleComponent))
  (bind _unitarray (Variables|Default|GetUnitArray))
  (bind _returnvalue (Transformation|GetWorldLocation _capsulecomponent))
  (bind (_distance _returnvalue_2) (Actor|FindNearestActor _returnvalue _unitarray))
  (if (Utilities|IsValid _returnvalue_2)
    (if (<= _distance (Math|Conversions|ToFloat(Integer) (Variables|Default|GetWeaponRange)))
      (bind _outhit (Collision|LineTraceByChannel _returnvalue (Transformation|GetActorLocation _returnvalue_2) "TraceTypeQuery1" false 0 "ForDuration"))
      (Class|RTSInterface|DealDamage(Message) (.HitActor (Collision|BreakHitResult _outhit)) (Variables|Default|GetWeaponDamage)))
    (elif true
      (if (<= (.Distance (Actor|FindNearestActor _returnvalue (stale EventTick _outactors))) (Math|Conversions|ToFloat(Integer) (Variables|Default|GetWeaponRange)))
        (bind _outhit_2 (Collision|LineTraceByChannel (Transformation|GetWorldLocation (Variables|Default|GetCapsuleComponent)) (Transformation|GetActorLocation (.ReturnValue (Actor|FindNearestActor _returnvalue (stale EventTick _outactors)))) "TraceTypeQuery1" false 0 "ForDuration"))
        (Class|RTSInterface|DealDamage(Message) (.HitActor (Collision|BreakHitResult _outhit_2)) (Variables|Default|GetWeaponDamage))))))

(event EventBeginPlay
  (bind _ashealth_bar (Utilities|Casting|CastToHealthBar (UserInterface|GetUserWidgetObject (Variables|Default|GetHealthBar))))
  (Variables|/Game/Blueprints/HUD/HealthBar.HealthBar_C|SetEnemyUnit _ashealth_bar self)
  (bind _outactors (Actor|GetAllActorsOfClass "/Game/Blueprints/Units/MyUnitAI.MyUnitAI_C"))
  (Variables|Default|SetUnitArray _outactors)
  (Utilities|Time|SetTimerbyEvent (delegate Custom|ShootUnit) (Variables|Default|GetWeaponFireRate) true))

(event EventTick
  (params (DeltaSeconds :type Float%20%28single-precision%29))
  (bind _unitarray (Variables|Default|GetUnitArray))
  (if (>= (Variables|Default|GetHealthPoints) 0)
    (if (Utilities|Array|IsValidIndex _unitarray)
      (for _array_element _unitarray
        (CallFunction|SetLocation _array_element)
        (AI|AIMoveTo self (Variables|Default|GetCustom%20Location) 0 1e+01 true
          (:OnSuccess
            (Variables|Default|SetClosestDistance 9e+05))))
      (else
        (bind _outactors (Actor|GetAllActorsOfClass "/Game/Blueprints/Buildings/Parent_Building_Class.Parent_Building_Class_C"))
        (for _array_element_2 _outactors
          (CallFunction|SetLocation _array_element_2)
          (AI|AIMoveTo self (Variables|Default|GetCustom%20Location) 0 1e+01 true
            (:OnSuccess
              (Variables|Default|SetClosestDistance 9e+05))))))
    (else
      (Actor|DestroyActor))))

(event EventDealDamage
  (params (Damage :type Integer))
  (Variables|Default|SetHealthPoints (- (Variables|Default|GetHealthPoints) Damage)))

(event EventUnitDestroyed
  (params (DestroyedUnit :type My%20Unit%20AI%20Object%20Reference))
  (Utilities|Array|RemoveItem (Variables|Default|GetUnitArray) DestroyedUnit))

(event EventUnitProduced
  (params (NewUnit :type My%20Unit%20AI%20Object%20Reference))
  (Utilities|Array|AddUnique (Variables|Default|GetUnitArray) NewUnit))

(fn ConstructionScript)

(fn Moving)

(fn CustomMoving
  (params (CustomLocation1 :type Vector)))

(fn SetLocation
  (params (TargetActor :type Actor%20Object%20Reference))
  (bind _returnvalue (Transformation|GetActorLocation TargetActor))
  (bind _returnvalue_2 (Transformation|GetActorLocation))
  (bind _returnvalue_3 (Math|Vector|Distance2D(Vector) _returnvalue _returnvalue_2))
  (if (Utilities|IsValid TargetActor)
    (if (< _returnvalue_3 (Variables|Default|GetClosestDistance))
      (Variables|Default|SetClosestDistance _returnvalue_3)
      (Variables|Default|SetCustom%20Location _returnvalue))))

(fn CanCapture
  (return false))

(fn GrabSelectedEnemies
  (return 0))

(fn GrabSelectedUnits
  (return 0))

(fn ResourceKeeper
  (return 0.0 0.0 0.0))